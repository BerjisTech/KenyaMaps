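; Wall builder actor that previews a grid of WallMesh copies and can turn them into individual StaticMeshActors.
; The construction script fills an InstancedStaticMesh in X and Z, stepping by mesh bounds; spacing values act as constant offsets, not per-step gaps.
; Each column gets a base instance plus its vertical loop instances.
; SpawnInPlace, gated by SpawnThem, spawns an actor at each instance's world transform, leaving the instances intact.
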(event EventBeginPlay)

(event Collision|EventActorBeginOverlap
  (params (OtherActor :type Actor%20Object%20Reference)))

(event EventTick
  (params (DeltaSeconds :type Float%20%28single-precision%29)))

(fn ConstructionScript
  (bind _wallmesh (Variables|Default|GetwallMesh))
  (Components|StaticMesh|SetStaticMesh (Variables|Default|GetInstancedStaticMesh) _wallmesh)
  (for _index (range 0 (Variables|Default|GethorizontalInstances))
    (Components|InstancedStaticMesh|AddInstance (Variables|Default|GetInstancedStaticMesh) (Math|Transform|MakeTransform (+ (Variables|/Script/Engine.SceneComponent|GetRelativeLocation (Variables|Default|GetInstancedStaticMesh)) (Math|Vector|MakeVector (+ (* (* (.x (.boxextent (StaticMesh|GetBounds _wallmesh))) 2.0) _index) (Variables|Default|GethorizontalSpacing)) 0.0 0.0)) "0, 0, 0" "1.000000,1.000000,1.000000") false)
    (for _index_2 (range 0 (Variables|Default|GetverticalInstances))
      (Components|InstancedStaticMesh|AddInstance (Variables|Default|GetInstancedStaticMesh) (Math|Transform|MakeTransform (+ (+ (Variables|/Script/Engine.SceneComponent|GetRelativeLocation (Variables|Default|GetInstancedStaticMesh)) (Math|Vector|MakeVector (+ (* (* (.x (.boxextent (StaticMesh|GetBounds _wallmesh))) 2.0) _index) (Variables|Default|GethorizontalSpacing)) 0.0 0.0)) (Math|Vector|MakeVector 0.0 0.0 (+ (* (* (.z (.boxextent (StaticMesh|GetBounds (Variables|Default|GetwallMesh)))) 2.0) _index_2) (Variables|Default|GetverticalSpacing)))) "0, 0, 0" "1.000000,1.000000,1.000000") false))))

(fn SpawninPlace
  (bind _instancedstaticmesh (Variables|Default|GetInstancedStaticMesh))
  (if (Variables|Default|GetspawnThem)
    (for _index (range 0 (- (Components|InstancedStaticMesh|GetInstanceCount _instancedstaticmesh) 1))
      (bind _returnvalue (Game|SpawnActorfromClass "/Script/Engine.StaticMeshActor" (.OutInstanceTransform (Components|InstancedStaticMesh|GetInstanceTransform _instancedstaticmesh _index true)) "Undefined" "MultiplyWithRoot" 0 0))
      (Components|StaticMesh|SetStaticMesh (Variables|/Script/Engine.StaticMeshActor|GetStaticMeshComponent _returnvalue) (Variables|Default|GetwallMesh)))))